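; BP_ArchVisController is a controller Blueprint for an architectural visualization plan tool, currently enabling only input debugging on BeginPlay.
; Disconnected, never-run logic would create an RTPlan tool manager from the shared document and cache its select tool.
; Another unused chain would build the wall properties widget, async-load the wall finish catalog, then pass document and catalog to the plan shell actor.
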(event EventBeginPlay
  (Utilities|FlowControl|Sequence
    (:then_0
      (Class|ArchVisPlayerController|SetInputDebugEnabled true))))

(fn ConstructionScript)